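; BP_GameModeLobby is a lobby game mode that acts as the hub for player chat and the player list.
; PostLogin stores each joining BP_PlayerControllerChat in an array.
; SendUpdateUIToClients rebuilds PlayerInfos from each controller's PlayerStatus and pushes it to all of them, while SendMessageToAll relays a message through each controller's AddMessage.
; A debug event prints nicknames, but its authority-gated looping timer is disconnected and never runs.
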(event `self.ReceiveBeginPlay`)

(event `TestPlayerNicknames`
  (for _array_element (`self.AllPlayerControllerChat`)
    (`KismetSystemLibrary.PrintString` (`/Game/Game/BP_PlayerControllerChat.Nickname` _array_element) true true (struct :`G` 0.66 :`B` 1.0 :`A` 1.0) 1.0)))

(event `self.K2_PostLogin`
  (params (NewPlayer :type "PlayerController Object Reference"))
  (bind _asbp_player_controller_chat (cast `/Game/Game/BP_PlayerControllerChat` NewPlayer))
  (`KismetArrayLibrary.Array_AddUnique` (`self.AllPlayerControllerChat`) _asbp_player_controller_chat))

(event `SendUpdateUIToClients`
  (bind _allplayercontrollerchat (`self.AllPlayerControllerChat`))
  (`KismetArrayLibrary.Array_Clear` (`self.PlayerInfos`))
  (for _array_element _allplayercontrollerchat
    (`KismetArrayLibrary.Array_AddUnique` (`self.PlayerInfos`) (`/Game/Game/BP_PlayerControllerChat.PlayerStatus` _array_element)))
  (for _array_element_2 _allplayercontrollerchat
    (`/Game/Game/BP_PlayerControllerChat.ClientUpdatePlayerlist` _array_element_2 (`self.PlayerInfos`))))

(event `SendMessageToAll`
  (params (Message :type Text))
  (for _array_element (`self.AllPlayerControllerChat`)
    (`/Game/Game/BP_PlayerControllerChat.AddMessage` _array_element Message)))

(fn `UserConstructionScript`)