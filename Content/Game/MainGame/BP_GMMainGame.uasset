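; Game mode for a multiplayer pumpkin-collecting match that runs player spawning and win/lose flow on the server.
; BeginPlay scatters pumpkins over random spawn points, and SpawnMe gives each requesting controller a character at an indexed PlayerStart.
; Tick sets the GameState's status to Playing once the lobby's player count has spawned.
; It then declares Lose when no player retains a character, or Win when their combined pumpkins reach the target.
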(event `self.K2_OnSwapPlayerControllers`
  (params (OldPC :type "PlayerController Object Reference") (NewPC :type "PlayerController Object Reference"))
  ;[0.3508 1 0] Wenn jemand dem game joined
  (`/Engine/EditorBlueprintResources/ActorMacros.Switch Has Authority`
    (:`Authority`
      (bind _asbp_pcmain_game (cast `/Game/Game/MainGame/BP_PCMainGame` NewPC))
      (`KismetArrayLibrary.Array_AddUnique` (`self.AllPlayer`) _asbp_pcmain_game)
      (`KismetSystemLibrary.PrintString` "Added" true true (struct :`G` 0.66 :`B` 1.0 :`A` 1.0) 30.0 :!label _label))))

(event `self.K2_PostLogin`
  (params (NewPlayer :type "PlayerController Object Reference"))
  ;[0.3508 1 0] Wenn jemand dem game joined
  (`/Engine/EditorBlueprintResources/ActorMacros.Switch Has Authority`
    (:`Authority`
      (bind _asbp_pcmain_game (cast `/Game/Game/MainGame/BP_PCMainGame` NewPlayer))
      (`KismetArrayLibrary.Array_AddUnique` (`self.AllPlayer`) _asbp_pcmain_game)
      (goto _label))))

(event `self.ReceiveTick`
  (params (DeltaSeconds :type "Float (single-precision)"))
  ;[1 0.3003 0] Event Tick check win lose condition
  (`/Engine/EditorBlueprintResources/ActorMacros.Switch Has Authority`
    (:`Authority`
      (bind _asbp_gsmain_game (cast `/Game/Game/MainGame/BP_GSMainGame` (`GameplayStatics.GetGameState`)))
      (switch `/Game/Game/MainGame/E_GSMainGame` (`/Game/Game/MainGame/BP_GSMainGame.GameStatus` _asbp_gsmain_game)
        (:`NewEnumerator3`
          (bind _asbp_my_game_instance (cast `/Game/Game/BP_MyGameInstance` (`GameplayStatics.GetGameInstance`)))
          (if (== (`self.JoinedPlayer`) (`/Game/Game/BP_MyGameInstance.NumPlayerInLobby` _asbp_my_game_instance))
            (bind _asbp_gsmain_game_2 (cast `/Game/Game/MainGame/BP_GSMainGame` (`GameplayStatics.GetGameState`)))
            (set `/Game/Game/MainGame/BP_GSMainGame.GameStatus` "NewEnumerator0" _asbp_gsmain_game_2)))
        (:`NewEnumerator0`
          (bind _alldead_ (`self.CheckGameOver`))
          (if _alldead_
            (`/Engine/EditorBlueprintResources/StandardMacros.DoOnce` false
              (:`Completed`
                (bind _asbp_gsmain_game_3 (cast `/Game/Game/MainGame/BP_GSMainGame` (`GameplayStatics.GetGameState`)))
                (set `/Game/Game/MainGame/BP_GSMainGame.GameStatus` "NewEnumerator2" _asbp_gsmain_game_3)))
            (else
              (bind _win_ (`self.CheckPumpkinsWin`))
              (if _win_
                (`/Engine/EditorBlueprintResources/StandardMacros.DoOnce` false
                  (:`Completed`
                    (bind _asbp_gsmain_game_4 (cast `/Game/Game/MainGame/BP_GSMainGame` (`GameplayStatics.GetGameState`)))
                    (set `/Game/Game/MainGame/BP_GSMainGame.GameStatus` "NewEnumerator1" _asbp_gsmain_game_4)))))))))))

(event `self.ReceiveBeginPlay`
  ;[1 0 0] On Begin play spawn pumpkins and player character and then start the game
  (`/Engine/EditorBlueprintResources/ActorMacros.Switch Has Authority`
    (:`Authority`
      (`KismetArrayLibrary.Array_Clear` (`self.AllPlayer`))
      (`self.SpawnPumpkins`))))

(event `SpawnPlayers`
  ;[1 0 0] Spawn player characters
)

(event `SpawnMe`
  (params (Controller :type "/Game/Game/MainGame/BP_PCMainGame Object Reference"))
  (bind _returnvalue (`Controller.K2_GetPawn` Controller))
  ;[1 1 1] Self call spawn my pawn
  (`/Engine/EditorBlueprintResources/ActorMacros.Switch Has Authority`
    (:`Authority`
      (`/Engine/EditorBlueprintResources/StandardMacros.IsValid` _returnvalue
        (:`Is Valid`
          (`self.K2_DestroyActor` _returnvalue))
        (:`Is Not Valid`
          _))
      (bind _location (`self.GetSpawnPoints` (`self.JoinedPlayer`)))
      (`/Engine/EditorBlueprintResources/StandardMacros.IncrementInt` (`self.JoinedPlayer`)
        (:`  `
          (bind _returnvalue_2 (`|SpawnActorFromClass` "/Game/ThirdPerson/Blueprints/BP_ThirdPersonCharacter.BP_ThirdPersonCharacter_C" (`KismetMathLibrary.MakeTransform` _location) "Undefined" "OverrideRootScale" null null))
          (`Controller.Possess` Controller _returnvalue_2))))))

(fn `CheckGameOver`
  (returns (`AllDead?` :type Boolean))
  (locals (AnzahlDead :type Integer))
  (bind _anzahldead (`local.AnzahlDead`))
  (set `local.AnzahlDead` 0)
  (for _array_element (`self.AllPlayer`)
    (cast `/Game/ThirdPerson/Blueprints/BP_ThirdPersonCharacter` (`Controller.K2_GetPawn` _array_element)
      (:`CastFailed`
        (`/Engine/EditorBlueprintResources/StandardMacros.IncrementInt` (`local.AnzahlDead`)))))
  (bind _asbp_my_game_instance (cast `/Game/Game/BP_MyGameInstance` (`GameplayStatics.GetGameInstance`)))
  (bind _numplayerinlobby (`/Game/Game/BP_MyGameInstance.NumPlayerInLobby` _asbp_my_game_instance))
  (`KismetSystemLibrary.PrintString` (`KismetStringLibrary.Concat_StrStr` "Spieler Tot: " (`KismetStringLibrary.Conv_IntToString` _anzahldead) ">= AnzahlSpieler:  " (`KismetStringLibrary.Conv_IntToString` _numplayerinlobby)))
  (return (>= _anzahldead _numplayerinlobby)))

(fn `CheckPumpkinsWin`
  (returns (`Win?` :type Boolean))
  (locals (AnzInsgesamtPumpkins :type Integer))
  (set `local.AnzInsgesamtPumpkins` 0)
  (for _array_element (`self.AllPlayer`)
    (bind _asbp_third_person_character (cast `/Game/ThirdPerson/Blueprints/BP_ThirdPersonCharacter` (`Controller.K2_GetPawn` _array_element)))
    (set `local.AnzInsgesamtPumpkins` (+ (`local.AnzInsgesamtPumpkins`) (`/Game/ThirdPerson/Blueprints/BP_ThirdPersonCharacter.Pumpkins` _asbp_third_person_character))))
  (return (>= (`local.AnzInsgesamtPumpkins`) 8)))

(fn `GetSpawnPoints`
  (params (index :type Integer))
  (returns (Location :type "Vector Structure"))
  (bind _outactors (`GameplayStatics.GetAllActorsOfClass` "/Script/Engine.PlayerStart"))
  (return (`self.K2_GetActorLocation` (`|GetArrayItem` _outactors index))))

(fn `SpawnPumpkins`
  (bind _outactors (`GameplayStatics.GetAllActorsOfClass` "/Game/Blueprints/BP_Spawnpoint.BP_Spawnpoint_C"))
  (set `self.SpawnReferences` _outactors)
  (for _ (range (`self.MaxPumpkinsNeeded`))
    (set `self.Item` (`KismetArrayLibrary.Array_Random` (`self.SpawnReferences`)))
    (`|SpawnActorFromClass` "/Game/Blueprints/BP_Pumpkin.BP_Pumpkin_C" (`KismetMathLibrary.MakeTransform` (`self.K2_GetActorLocation` (`self.Item`))) "AdjustIfPossibleButAlwaysSpawn" "OverrideRootScale" null null)
    (`KismetArrayLibrary.Array_RemoveItem` (`self.SpawnReferences`) (`self.Item`))
    (`self.K2_DestroyActor` (`self.Item`))))

(fn `UserConstructionScript`)