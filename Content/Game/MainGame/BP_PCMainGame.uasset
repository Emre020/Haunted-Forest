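; BP_PCMainGame is the main game's player controller, which sets up the local UI and asks the game mode to spawn it.
; On BeginPlay the local controller clears existing widgets, shows WBP_ShowPumpkin and switches to game-only input.
; After a short delay, ReadyToSpawn calls LikeToSpawn, which passes the controller to BP_GMMainGame's SpawnMe, printing an error if the game mode cast fails.
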(event `self.ReceiveBeginPlay`
  (`|ExecutionSequence`
    (:`then_0`
      (if (`self.IsLocalController`)
        (`WidgetLayoutLibrary.RemoveAllWidgets`)
        (bind _returnvalue (`|CreateWidget` "/Game/Blueprints/UI/WBP_ShowPumpkin.WBP_ShowPumpkin_C"))
        (`UserWidget.AddToViewport` _returnvalue 0)
        (`WidgetBlueprintLibrary.SetInputMode_GameOnly` self)))
    (:`then_1`
      (`KismetSystemLibrary.Delay` 0.2)
      (`self.ReadyToSpawn`))))

(event `ReadyToSpawn`
  (`self.LikeToSpawn`))

(event `LikeToSpawn`
  (bind _asbp_gmmain_game (cast `/Game/Game/MainGame/BP_GMMainGame` (`GameplayStatics.GetGameMode`))
    (:`then`
      (`/Game/Game/MainGame/BP_GMMainGame.SpawnMe` _asbp_gmmain_game self))
    (:`CastFailed`
      (`KismetSystemLibrary.PrintString` "FAIL!!!!!! Cast to game mode failed!" true true (struct :`R` 1.0 :`A` 1.0) 30.0))))

(fn `UserConstructionScript`)