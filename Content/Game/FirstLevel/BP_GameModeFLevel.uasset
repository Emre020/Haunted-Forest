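; Game mode for the first level that handles player respawns and enemy AI spawning.
; BeginPlay sets the game status and starts a looping timer spawning BP_KIGegner at random reachable points, each targeting a random player.
; Controllers register on PostLogin or controller swap, which carries over chat-controller player info and nickname.
; Authority Tick respawns dead or pawnless players at index-tagged PlayerStarts in their color; the delayed start sequence is disconnected.
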(event `self.ReceiveTick`
  (params (DeltaSeconds :type "Float (single-precision)"))
  (`/Engine/EditorBlueprintResources/ActorMacros.Switch Has Authority`
    (:`Authority`
      (`self.CheckHealth`))))

(event `self.ReceiveBeginPlay`
  ;[1 1 1] On Begin Play Change status and dealayed start
  (bind _asbp_game_state_flevel (cast `/Game/Game/FirstLevel/BP_GameStateFLevel` (`GameplayStatics.GetGameState`)))
  (set `/Game/Game/FirstLevel/BP_GameStateFLevel.GameStatus` "NewEnumerator1" _asbp_game_state_flevel)
  (`KismetSystemLibrary.K2_SetTimerDelegate` (delegate `SpawnKI`) 5.0 true))

(event `SpawnKI`
  ;[1 1 1] Spawn KI
  (`/Engine/EditorBlueprintResources/ActorMacros.Switch Has Authority`
    (:`Authority`
      (bind _returnvalue (`AIBlueprintHelperLibrary.SpawnAIFromClass` "/Game/Blueprints/BP_KIGegner.BP_KIGegner_C" null (`NavigationSystemV1.K2_GetRandomReachablePointInRadius` (0.0 0.0 0.0) 5000.0 null null) (struct) false self))
      (`KismetSystemLibrary.Delay` 0.2)
      (bind _asbp_kigegner (cast `/Game/Blueprints/BP_KIGegner` _returnvalue))
      (set `/Game/Blueprints/BP_KIGegner.AttackGoal` (`GameplayStatics.GetPlayerPawn` (`KismetMathLibrary.RandomIntegerInRange` 0 (- (`GameplayStatics.GetNumPlayerControllers`) 1))) _asbp_kigegner))))

(event `SpawnPlayersAndPossess`
  ;[1 1 1] Spawn all player an possess
  (for (_array_element _array_index) (`self.AllPlayerControllers`)
    (bind _returnvalue (`Controller.K2_GetPawn` _array_element))
    (`/Engine/EditorBlueprintResources/StandardMacros.IsValid` _returnvalue
      (:`Is Valid`
        (`self.K2_DestroyActor` _returnvalue))
      (:`Is Not Valid`
        _))
    (bind _position (`self.GetPlayerStartLocation` _array_index))
    (bind (_playerstatus_isready _playerstatus_nickname _playerstatus_color _playerstatus_colorlinear) (break `/Game/Blueprints/S_PlayerStatus` (`/Game/Game/FirstLevel/BP_PlayerControllerFLevel.PlayerStatus` _array_element)))
    (bind _returnvalue_2 (`|SpawnActorFromClass` "/Game/Blueprints/BP_MyTPCharacter.BP_MyTPCharacter_C" (`KismetMathLibrary.MakeTransform` _position) "Undefined" "OverrideRootScale" _array_element _playerstatus_colorlinear null))
    (`Controller.Possess` _array_element _returnvalue_2)))

(event `self.K2_PostLogin`
  (params (NewPlayer :type "PlayerController Object Reference"))
  ;[1 1 1] Nur zum debuggen
  (bind _asbp_player_controller_flevel (cast `/Game/Game/FirstLevel/BP_PlayerControllerFLevel` NewPlayer))
  (`KismetArrayLibrary.Array_AddUnique` (`self.AllPlayerControllers`) _asbp_player_controller_flevel))

(event `self.K2_OnSwapPlayerControllers`
  (params (OldPC :type "PlayerController Object Reference") (NewPC :type "PlayerController Object Reference"))
  ;[1 1 1] On Join forward player infos like color, name...  and save them
  (bind _asbp_player_controller_chat (cast `/Game/Game/BP_PlayerControllerChat` OldPC))
  (bind _asbp_player_controller_flevel (cast `/Game/Game/FirstLevel/BP_PlayerControllerFLevel` NewPC))
  (bind _output_get (set `/Game/Game/FirstLevel/BP_PlayerControllerFLevel.PlayerStatus` (`/Game/Game/BP_PlayerControllerChat.PlayerStatus` _asbp_player_controller_chat) _asbp_player_controller_flevel))
  (`KismetArrayLibrary.Array_AddUnique` (`self.AllPlayerControllers`) _asbp_player_controller_flevel)
  ;[1 1 1] Setzte direkt den Nickname
  (bind _asbp_player_state_flevel (cast `/Game/Game/FirstLevel/BP_PlayerStateFLevel` (`Controller.PlayerState` _asbp_player_controller_flevel)))
  (set `/Game/Game/FirstLevel/BP_PlayerStateFLevel.Nickname` (`.Nickname_5_F74F828745B9F92BD23D7F93DCDCC1C9` (break `/Game/Blueprints/S_PlayerStatus` _output_get)) _asbp_player_state_flevel))

(fn `CheckHealth`
  (for (_array_element _array_index) (`self.AllPlayerControllers`)
    (bind _returnvalue (`Controller.K2_GetPawn` _array_element))
    (`/Engine/EditorBlueprintResources/StandardMacros.IsValid` _returnvalue
      (:`Is Valid`
        (bind _asbp_my_tpcharacter (cast `/Game/Blueprints/BP_MyTPCharacter` _returnvalue))
        (if (<= (`/Game/Blueprints/BP_MyTPCharacter.Health` _asbp_my_tpcharacter) 0.0)
          (`self.K2_DestroyActor` _asbp_my_tpcharacter)
          (bind _position (`self.GetPlayerStartLocation` _array_index :!label _label))
          (bind (_playerstatus_isready _playerstatus_nickname _playerstatus_color _playerstatus_colorlinear) (break `/Game/Blueprints/S_PlayerStatus` (`/Game/Game/FirstLevel/BP_PlayerControllerFLevel.PlayerStatus` _array_element)))
          (bind _returnvalue_2 (`|SpawnActorFromClass` "/Game/Blueprints/BP_MyTPCharacter.BP_MyTPCharacter_C" (`KismetMathLibrary.MakeTransform` _position) "Undefined" "OverrideRootScale" null _playerstatus_colorlinear null))
          (`Controller.Possess` _array_element _returnvalue_2)))
      (:`Is Not Valid`
        (goto _label)))))

(fn `GetPlayerStartLocation`
  (params (index :type Integer))
  (returns (Position :type "Vector Structure"))
  (bind _outactors (`GameplayStatics.GetAllActorsOfClass` "/Script/Engine.PlayerStart"))
  (for _array_element _outactors
    (if (== (`PlayerStart.PlayerStartTag` _array_element) (`KismetStringLibrary.Conv_StringToName` (`KismetStringLibrary.Conv_IntToString` index)))
      (return (`self.K2_GetActorLocation` _array_element)))))

(fn `UserConstructionScript`)